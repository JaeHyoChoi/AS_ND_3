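; BP_ChoiceCube is an actor whose static mesh shuttles between its initial relative location and that of TargetComponent.
; On Tick, IsWaitCube selects either nonstop movement or a mode that pauses three seconds after each leg.
; Both modes share LenthCheck to measure travel, Shufle to swap endpoints on arrival, and MoveUpdate to step the mesh by Speed and delta time without sweeping.
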(event EventBeginPlay
  (Variables|Default|SetStartLocation (Variables|/Script/Engine.SceneComponent|GetRelativeLocation (Variables|Default|GetStaticMesh)))
  (Variables|Default|SetTargetLocation (Variables|/Script/Engine.SceneComponent|GetRelativeLocation (Variables|Default|GetTargetComponent))))

(event EventTick
  (params (DeltaSeconds :type Float%20%28single-precision%29))
  (if (Variables|Default|GetIsWaitCube)
    (CallFunction|WaitMove DeltaSeconds)
    (else
      (CallFunction|DontStopMove DeltaSeconds))))

(fn ConstructionScript)

(fn MoveUpdate
  (params (DeltaTime :type Float%20%28double-precision%29))
  ;[1 1 1] 이동
  (Transformation|SetRelativeLocation (Variables|Default|GetStaticMesh) (+ (Variables|/Script/Engine.SceneComponent|GetRelativeLocation (Variables|Default|GetStaticMesh)) (* (Math|Vector|Normalize (- (Variables|Default|GetTargetLocation) (Variables|Default|GetStartLocation))) (* (Variables|Default|GetSpeed) DeltaTime))) false false))

(fn LenthCheck
  ;[1 1 1] 가야할 거리
  (Variables|Default|SetLenth (Math|Vector|VectorLength (- (Variables|Default|GetTargetLocation) (Variables|Default|GetStartLocation))))
  ;[1 1 1] 가고 있는 거리
  (Variables|Default|SetTravelled (Math|Vector|VectorLength (- (Variables|/Script/Engine.SceneComponent|GetRelativeLocation (Variables|Default|GetStaticMesh)) (Variables|Default|GetStartLocation)))))

(fn Shufle
  ;[1 1 1] 위치 셔플 바꾸기
  (if (>= (Variables|Default|GetTravelled) (Variables|Default|GetLenth))
    (Variables|Default|SetTempLocation (Variables|Default|GetStartLocation))
    (Variables|Default|SetStartLocation (Variables|Default|GetTargetLocation))
    (Variables|Default|SetTargetLocation (Variables|Default|GetTempLocation))
    (return true)
    (else
      (return false))))

(fn WaitTimeCheck
  (params (DeltaTime :type Float%20%28double-precision%29))
  (bind _output_get (Variables|Default|SetAcctime (+ (Variables|Default|GetAcctime) DeltaTime)))
  (if (>= _output_get 3.0)
    (Variables|Default|SetIsWait false)
    (Variables|Default|SetAcctime 0.0)))

(fn WaitMove
  (params (DeltaTime :type Float%20%28double-precision%29))
  (if (Variables|Default|GetIsWait)
    (CallFunction|WaitTimeCheck DeltaTime)
    (else
      (CallFunction|LenthCheck)
      (bind _ischange (CallFunction|Shufle))
      (Variables|Default|SetIsWait _ischange)
      (CallFunction|MoveUpdate DeltaTime))))

(fn DontStopMove
  (params (DeltaTime :type Float%20%28double-precision%29))
  (CallFunction|LenthCheck)
  (CallFunction|Shufle)
  (CallFunction|MoveUpdate DeltaTime))